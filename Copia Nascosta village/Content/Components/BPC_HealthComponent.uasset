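; BPC_HealthComponent is a health component that applies damage to the health of its owning actor.
; RealizesDamage subtracts damage from current health and clamps the result between zero and max health.
; Non-lethal hits call DamageHasBeenDone, while reaching zero only prints Spanish debug messages and the health value, with no further death handling.
; BeginPlay and Tick are unused.
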(fn `RealizesDamage`
  (params (Damage :type "Float (double-precision)"))
  (bind _output_get (set `self.CurrentsHealth` (`KismetMathLibrary.FClamp` (- (`self.CurrentsHealth`) Damage) 0.0 (`self.MaxHealth`))))
  (if (== _output_get 0.0)
    (`KismetSystemLibrary.PrintString` "El actor llego a 0  *se murio*")
    (`KismetSystemLibrary.PrintString` (`KismetStringLibrary.Conv_DoubleToString` _output_get))
    (else
      (`KismetSystemLibrary.PrintString` "Se quito vida.")
      (`self."Damage has been done"`))))