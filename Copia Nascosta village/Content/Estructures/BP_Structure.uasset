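; BP_Structure is a demonstration Blueprint that stores player stats in a StatsBar struct and shows them on screen.
; BeginPlay prints the struct's health, experience, user name and abilities enum, waits, then calls SetStructure.
; SetStructure overwrites the whole struct with hardcoded values and prints the same fields again to show the change.
; The "Vida Actual" (current health) label displays MaximusHealth, and the construction script is empty.
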(event `self.ReceiveBeginPlay`
  (bind (_stats_bar_maximushealth _stats_bar_experience _stats_bar_username _stats_bar_habilities) (break `/Game/Estructures/BPS_Stats` (`self.Stats Bar`)))
  (`KismetSystemLibrary.PrintString` (`KismetStringLibrary.Concat_StrStr` " \nVida Actual: \n " (`KismetStringLibrary.Conv_DoubleToString` _stats_bar_maximushealth) " \nExperiencia:     \n" (`KismetStringLibrary.Conv_DoubleToString` _stats_bar_experience) " \nNombre:    \n" _stats_bar_username " \nHabilidades: \n" (`|GetEnumeratorNameAsString` _stats_bar_habilities)) true true (struct :`R` 1.0 :`G` 0.088973 :`B` 0.680636 :`A` 1.0) 5.0)
  (`KismetSystemLibrary.Delay` 10.0)
  (`self.Set Structure`))

(event `Set Structure`
  (bind _output_get (set `self.Stats Bar` (make `/Game/Estructures/BPS_Stats` 5.0)))
  (`KismetSystemLibrary.PrintString` (`KismetStringLibrary.Concat_StrStr` " \nVida Actual: \n " (`KismetStringLibrary.Conv_DoubleToString` (break `/Game/Estructures/BPS_Stats` _output_get)) " \nExperiencia:     \n" (`KismetStringLibrary.Conv_DoubleToString` (`.Experience_18_E372BE3A480C7B35D072D9813B302446` (break `/Game/Estructures/BPS_Stats` _output_get))) " \nNombre:    \n" (`.UserName_15_BA311BCF4E3DE7A6B1F954A26CD87C4F` (break `/Game/Estructures/BPS_Stats` _output_get)) " \nHabilidades: \n" (`|GetEnumeratorNameAsString` (`.Habilities_16_E9200E424E70FFA6E2BF6198279352C3` (break `/Game/Estructures/BPS_Stats` _output_get)))) true true (struct :`R` 1.0 :`G` 0.088973 :`B` 0.680636 :`A` 1.0) 5.0)
  (`KismetSystemLibrary.Delay` 10.0))

(fn `UserConstructionScript`)