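; BP_character is the player character, handling movement input and contact damage to actors it overlaps.
; On BeginPlay it adds the default Enhanced Input mapping context, and IA_Move feeds movement along fixed world X and Y axes, independent of camera or control rotation.
; On overlap, it looks for BPC_HealthComponent on the other actor and, if found, passes its Damage value to RealizesDamage.
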(event `self.ReceiveBeginPlay`
  (bind _asplayer_controller (cast `PlayerController` (`self.GetController`)))
  (`EnhancedInputSubsystemInterface.AddMappingContext` (pcsubsystem `EnhancedInputLocalPlayerSubsystem` _asplayer_controller) "/Game/Character/Assets/Imputs/IMC_Default.IMC_Default" 0 (struct)))

(event `self.ReceiveActorBeginOverlap`
  (params (OtherActor :type "Actor Object Reference"))
  (bind _returnvalue (`self.GetComponentByClass` OtherActor "/Game/Components/BPC_HealthComponent.BPC_HealthComponent_C"))
  (`/Engine/EditorBlueprintResources/StandardMacros.IsValid` _returnvalue
    (:`Is Valid`
      (`/Game/Components/BPC_HealthComponent.RealizesDamage` _returnvalue (`self.Damage`)))))

(event `EnhancedInput|/Game/Character/Assets/Imputs/Actions/IA_Move`
  (params (ActionValue :type "Vector2D Structure") (ElapsedSeconds :type "Float (double-precision)") (TriggeredSeconds :type "Float (double-precision)") (InputAction :type "InputAction Object Reference" :default "/Game/Character/Assets/Imputs/Actions/IA_Move.IA_Move"))
  (:`Triggered`
    (`self.AddMovementInput` (1.0 0.0 0.0) ActionValue_X)
    (`self.AddMovementInput` (0.0 1.0 0.0) ActionValue_Y)))

(fn `UserConstructionScript`
  (`parent.UserConstructionScript`))