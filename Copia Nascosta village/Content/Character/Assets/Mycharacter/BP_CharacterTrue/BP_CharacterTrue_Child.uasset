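; Child player character that moves on world axes, switches between Idle, Melee and Ranged states, and fires projectiles toward the cursor.
; Enhanced Input drives movement, state changes and shooting, which yaws the actor to the cursor hit point before spawning BP_Proyectile.
; Entering Ranged immediately fires and destroys the actor, while the shoot input fires in any state.
; Overlaps damage actors with BPC_HealthComponent, and the death event only prints debug text.
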(event `self.ReceiveBeginPlay`
  (`parent.ReceiveBeginPlay`)
  (bind _asplayer_controller (cast `PlayerController` (`self.GetController`)))
  (`EnhancedInputSubsystemInterface.AddMappingContext` (pcsubsystem `EnhancedInputLocalPlayerSubsystem` _asplayer_controller) "/Game/Character/Assets/Imputs/IMC_Default.IMC_Default" 0 (struct)))

(event `EnhancedInput|/Game/Character/Assets/Imputs/Actions/IA_Move`
  (params (ActionValue :type "Vector2D Structure") (ElapsedSeconds :type "Float (double-precision)") (TriggeredSeconds :type "Float (double-precision)") (InputAction :type "InputAction Object Reference" :default "/Game/Character/Assets/Imputs/Actions/IA_Move.IA_Move"))
  (:`Triggered`
    (`self.AddMovementInput` (1.0 0.0 0.0) ActionValue_X)
    (`self.AddMovementInput` (0.0 1.0 0.0) ActionValue_Y)))

(event `self.ReceiveActorBeginOverlap`
  (params (OtherActor :type "Actor Object Reference"))
  (bind _returnvalue (`self.GetComponentByClass` OtherActor "/Game/Components/BPC_HealthComponent.BPC_HealthComponent_C"))
  (`/Engine/EditorBlueprintResources/StandardMacros.IsValid` _returnvalue
    (:`Is Valid`
      (`/Game/Components/BPC_HealthComponent.Realizes Damage` _returnvalue (`self.Damage_0`)))))

(event `Dead_1`
  (`KismetSystemLibrary.PrintString` "Hola acabo de Overaidear" true true (struct :`R` 1.0 :`G` 0.119738 :`A` 1.0) 10.0))

(event `self.UpdateUI`
  (`parent.UpdateUI`))

(event `EnhancedInput|/Game/Character/Assets/Imputs/Actions/IA_StateIddle`
  (params (ActionValue :type Boolean) (ElapsedSeconds :type "Float (double-precision)") (TriggeredSeconds :type "Float (double-precision)") (InputAction :type "InputAction Object Reference" :default "/Game/Character/Assets/Imputs/Actions/IA_StateIddle.IA_StateIddle"))
  (:`Started`
    (set `self.State` "NewEnumerator0")
    (`KismetSystemLibrary.PrintString` "Cambie a modo Iddle" true true (struct :`G` 0.034078 :`B` 1.0 :`A` 1.0))
    (set `PlayerController.bShowMouseCursor` false (`GameplayStatics.GetPlayerController` 0))))

(event `EnhancedInput|/Game/Character/Assets/Imputs/Actions/IA_StateMelee`
  (params (ActionValue :type Boolean) (ElapsedSeconds :type "Float (double-precision)") (TriggeredSeconds :type "Float (double-precision)") (InputAction :type "InputAction Object Reference" :default "/Game/Character/Assets/Imputs/Actions/IA_StateMelee.IA_StateMelee"))
  (:`Started`
    (set `self.State` "NewEnumerator1")
    (`KismetSystemLibrary.PrintString` "Cambie a modo Melee" true true (struct :`R` 1.0 :`A` 1.0))))

(event `EnhancedInput|/Game/Character/Assets/Imputs/Actions/IA_StateRanged`
  (params (ActionValue :type "Vector2D Structure") (ElapsedSeconds :type "Float (double-precision)") (TriggeredSeconds :type "Float (double-precision)") (InputAction :type "InputAction Object Reference" :default "/Game/Character/Assets/Imputs/Actions/IA_StateRanged.IA_StateRanged"))
  (:`Started`
    (bind _output_get (set `self.State` "NewEnumerator2"))
    (`KismetSystemLibrary.PrintString` "Cambie a modo Rango" true true (struct :`R` 1.0 :`G` 0.74805 :`B` 0.020335 :`A` 1.0))
    (set `PlayerController.bShowMouseCursor` false (`GameplayStatics.GetPlayerController` 0))
    (switch `/Game/Character/Enumeracion/E_Status` _output_get
      (:`NewEnumerator2`
        (`self.Shoting Projectil`)
        (`self.K2_DestroyActor`)))))

(event `EnhancedInput|/Game/Character/Assets/Imputs/Actions/IA_Shotting`
  (params (ActionValue :type "Vector2D Structure") (ElapsedSeconds :type "Float (double-precision)") (TriggeredSeconds :type "Float (double-precision)") (InputAction :type "InputAction Object Reference" :default "/Game/Character/Assets/Imputs/Actions/IA_Shotting.IA_Shotting"))
  (:`Started`
    (if true
      (`self.Shoting Projectil`)
      (set `PlayerController.bShowMouseCursor` true (`GameplayStatics.GetPlayerController` 0)))))

(fn `Shoting Projectil`
  (bind (_returnvalue_roll _returnvalue_pitch _returnvalue_yaw) (`KismetMathLibrary.BreakRotator` (`KismetMathLibrary.FindLookAtRotation` (`KismetMathLibrary.MakeVector` 0.0) (- (`.ImpactPoint` (`GameplayStatics.BreakHitResult` (`PlayerController.GetHitResultUnderCursorByChannel` (`GameplayStatics.GetPlayerController` 0) "TraceTypeQuery1" true))) (`self.K2_GetActorLocation`)))))
  (`self.K2_SetActorRotation` (`KismetMathLibrary.MakeRotator` 0.0 0.0 _returnvalue_yaw))
  (`|SpawnActorFromClass` "/Game/Blueprints/Props/Balas/BP_Proyectile.BP_Proyectile_C" (`self.GetTransform`) "Undefined" "MultiplyWithRoot" null 800.0 (0.0 0.0 0.0) null))

(fn `UserConstructionScript`
  (`parent.UserConstructionScript`))